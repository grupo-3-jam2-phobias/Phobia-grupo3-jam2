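; Interactive oxygen pickup that restores the player's oxygen by setting the game mode's 02NOSE value to a fixed amount.
; On BeginPlay it spawns attenuated, pitched-down music at its location.
; Its TriggerBoxO2 enables input on overlap and disables it on exit, without filtering the overlapping actor.
; Pressing E while enabled sets the oxygen value, destroys the actor and plays a 2D balloon sound.
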(event `self.ReceiveBeginPlay`
  (`GameplayStatics.SpawnSoundAtLocation` "/Game/StarterContent/Audio/Starter_Music01.Starter_Music01" (`self.K2_GetActorLocation`) (struct) 0.6 0.5 0.0 "/Game/Sonidos/MusOx.MusOx" null))

(event `Key|E`
  (params (Key :type "Key Structure"))
  (:`Pressed`
    (bind _asbp_third_person_game_mode (cast `/Game/ThirdPerson/Blueprints/BP_ThirdPersonGameMode` (`GameplayStatics.GetGameMode`)))
    (set `/Game/ThirdPerson/Blueprints/BP_ThirdPersonGameMode.02NOSE` 500.0 _asbp_third_person_game_mode)
    (`self.K2_DestroyActor`)
    (`GameplayStatics.PlaySound2D` "/Game/Sonidos/efectos/sonido_globo.sonido_globo" 1.0 1.0 0.0 null null)))

(event `self.Trigger Box O2.OnComponentBeginOverlap`
  (params (OverlappedComponent :type "PrimitiveComponent Object Reference") (OtherActor :type "Actor Object Reference") (OtherComp :type "PrimitiveComponent Object Reference") (OtherBodyIndex :type Integer) (bFromSweep :type Boolean) (SweepResult :type "HitResult Structure (by ref)"))
  (`self.EnableInput` (`GameplayStatics.GetPlayerController` 0)))

(event `self.Trigger Box O2.OnComponentEndOverlap`
  (params (OverlappedComponent :type "PrimitiveComponent Object Reference") (OtherActor :type "Actor Object Reference") (OtherComp :type "PrimitiveComponent Object Reference") (OtherBodyIndex :type Integer))
  (`self.DisableInput` (`GameplayStatics.GetPlayerController` 0)))

(fn `UserConstructionScript`)