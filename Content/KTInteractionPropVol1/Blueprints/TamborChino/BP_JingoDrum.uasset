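; Collectable Jingo drum prop that the player picks up by pressing E while inside its trigger box.
; Overlapping TriggerBoxR enables the actor's input for the first player controller, and leaving disables it, with no check on which actor overlaps.
; Pressing E decrements CollectablesLeft on BP_ThirdPersonGameMode, destroys the drum and plays a 2D sound.
; A positional Sonar sound node is left unconnected and never runs.
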(event `self.ReceiveBeginPlay`)

(event `Key|E`
  (params (Key :type "Key Structure"))
  (:`Pressed`
    (bind _asbp_third_person_game_mode (cast `/Game/ThirdPerson/Blueprints/BP_ThirdPersonGameMode` (`GameplayStatics.GetGameMode`)))
    (bind _result (`/Engine/EditorBlueprintResources/StandardMacros.DecrementInt` (`/Game/ThirdPerson/Blueprints/BP_ThirdPersonGameMode.CollectablesLeft` _asbp_third_person_game_mode))
      (:`  `
        (set `/Game/ThirdPerson/Blueprints/BP_ThirdPersonGameMode.CollectablesLeft` _result _asbp_third_person_game_mode)
        (`self.K2_DestroyActor`)
        (`GameplayStatics.PlaySound2D` "/Game/Sonidos/UI/hoverePum.hoverePum" 1.0 1.0 0.0 null null)))))

(event `self.Trigger Box R.OnComponentBeginOverlap`
  (params (OverlappedComponent :type "PrimitiveComponent Object Reference") (OtherActor :type "Actor Object Reference") (OtherComp :type "PrimitiveComponent Object Reference") (OtherBodyIndex :type Integer) (bFromSweep :type Boolean) (SweepResult :type "HitResult Structure (by ref)"))
  (`self.EnableInput` (`GameplayStatics.GetPlayerController` 0)))

(event `self.Trigger Box R.OnComponentEndOverlap`
  (params (OverlappedComponent :type "PrimitiveComponent Object Reference") (OtherActor :type "Actor Object Reference") (OtherComp :type "PrimitiveComponent Object Reference") (OtherBodyIndex :type Integer))
  (`self.DisableInput` (`GameplayStatics.GetPlayerController` 0)))

(fn `UserConstructionScript`)