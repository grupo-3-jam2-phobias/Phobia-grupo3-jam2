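; Ship (Nave) actor that acts as the end-of-game interaction point, gated on collectables, and emits an attenuated sonar sound from BeginPlay.
; Its trigger box enables player input only while overlapped, so pressing E checks CollectablesLeft on BP_ThirdPersonGameMode.
; At zero it pauses the game, adds the MuerteMenu and CinFI widgets and destroys itself.
; Otherwise it plays a dialogue line, with a flag and delay blocking repeat presses.
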(event `Key|E`
  (params (Key :type "Key Structure"))
  (:`Pressed`
    (if (not (`self.IsPlayngSound`))
      (set `self.IsPlayngSound` true)
      (bind _asbp_third_person_game_mode (cast `/Game/ThirdPerson/Blueprints/BP_ThirdPersonGameMode` (`GameplayStatics.GetGameMode`)))
      (if (== (`/Game/ThirdPerson/Blueprints/BP_ThirdPersonGameMode.CollectablesLeft` _asbp_third_person_game_mode) 0)
        (`GameplayStatics.SetGamePaused` true)
        (bind _returnvalue (`|CreateWidget` "/Game/UI/Menues/MuerteMenu.MuerteMenu_C"))
        (`UserWidget.AddToViewport` _returnvalue 0)
        (`self.K2_DestroyActor`)
        (bind _returnvalue_2 (`|CreateWidget` "/Game/Movies/CinFI.CinFI_C"))
        (`UserWidget.AddToViewport` _returnvalue_2 0)
        (else
          (`GameplayStatics.PlaySound2D` "/Game/Sonidos/Dialogo_2.Dialogo_2" 1.0 1.0 0.0 null null)))
      (`KismetSystemLibrary.Delay` 9.0)
      (set `self.IsPlayngSound` false))))

(event `self.Trigger Box R.OnComponentBeginOverlap`
  (params (OverlappedComponent :type "PrimitiveComponent Object Reference") (OtherActor :type "Actor Object Reference") (OtherComp :type "PrimitiveComponent Object Reference") (OtherBodyIndex :type Integer) (bFromSweep :type Boolean) (SweepResult :type "HitResult Structure (by ref)"))
  (`self.EnableInput` (`GameplayStatics.GetPlayerController` 0)))

(event `self.Trigger Box R.OnComponentEndOverlap`
  (params (OverlappedComponent :type "PrimitiveComponent Object Reference") (OtherActor :type "Actor Object Reference") (OtherComp :type "PrimitiveComponent Object Reference") (OtherBodyIndex :type Integer))
  (`self.DisableInput` (`GameplayStatics.GetPlayerController` 0)))

(event `self.ReceiveBeginPlay`
  (`GameplayStatics.SpawnSoundAtLocation` "/Game/Sonidos/Sonar/Sonar.Sonar" (`self.K2_GetActorLocation`) (struct) 1.0 1.0 0.0 "/Game/Sonidos/MusOx.MusOx" null))

(fn `UserConstructionScript`)