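; Enemy character that patrols random navigable points and chases pawns it sees.
; A successful AI move picks the next patrol point, keeping the loop going.
; Each sighting issues a move toward the pawn, with a DoOnce-gated switch of animation and walk speed.
; A retriggerable delay detects lost sight, then changes animation and speed, resets the gate and resumes patrol.
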(event `self.ReceiveBeginPlay`
  ;[1 1 1] Inicia el patrullaje (Al darle play)
  (`self.MoveToRandomLocation`))

(event `MoveToRandomLocation`
  ;[0.2104 0.5208 1] Patrullaje (cambiar radio)
  (bind _randomlocation (`NavigationSystemV1.K2_GetRandomLocationInNavigableRadius` (`self.K2_GetActorLocation`) 1200.0 null null))
  (`|AIMoveTo` self _randomlocation null 1200.0
    (:`OnSuccess`
      (`self.MoveToRandomLocation`))))

(event `self.ArcoDeVisión.OnSeePawn`
  (params (Pawn :type "Pawn Object Reference"))
  ;[0.1506 1 0.5258] Persecución
  (`|ExecutionSequence`
    (:`then_0`
      ;;[0.5223 0.204 1] Enemigo Alertado
      (`/Engine/EditorBlueprintResources/StandardMacros.DoOnce` false :!label _label
        (:`Completed`
          ;;;[1 0 0] MODIFICAR ANIMACIÓN
          (`SkeletalMeshComponent.PlayAnimation` (`self.Mesh`) "/Game/Characters/Mannequins/Animations/Manny/BS_MM_WalkRun.BS_MM_WalkRun" true)
          (set `CharacterMovementComponent.MaxWalkSpeed` 130.0 (`self.CharacterMovement`)))))
    (:`then_1`
      ;;[0.2027 0.6159 1] Enemigo Vuelve A Patrullar (pierde de vista al player)
      (`|AIMoveTo` self (0.0 0.0 0.0) Pawn 1200.0
        (:`then`
          ;;;[1 0 0] MODIFICAR VALOR
          (`KismetSystemLibrary.RetriggerableDelay` 2.0)
          ;;;[1 0 0] MODIFICAR ANIMACIÓN
          (`SkeletalMeshComponent.PlayAnimation` (`self.Mesh`) "/Game/Characters/Mannequins/Animations/Quinn/BS_MF_Unarmed_WalkRun.BS_MF_Unarmed_WalkRun" false)
          (set `CharacterMovementComponent.MaxWalkSpeed` 200.0 (`self.CharacterMovement`))
          (`self.CanSprintAgain`)
          (`self.MoveToRandomLocation`))))))

(event `CanSprintAgain`
  ;[0.1506 1 0.5258] Persecución
  ;;[0.5223 0.204 1] Enemigo Alertado
  (goto _label :!via `Reset`))

(fn `UserConstructionScript`)