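; BP_IndianShark is an enemy AI character that can patrol, chase and attack, and ends the game on touch.
; ChasePlayer repeats AIMoveTo toward player 0 after each successful move.
; Attack plays a montage and signals its end; helpers expose the patrol route and map speed states to walk speed.
; Box overlap with BP_ThirdPersonCharacter destroys the player controller and shows the MuerteMenu death screen.
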(event `self.ReceiveBeginPlay`)

(event `ChasePlayer`
  (`|AIMoveTo` self (0.0 0.0 0.0) (`GameplayStatics.GetPlayerCharacter` 0) 150.0
    (:`OnSuccess`
      (`KismetSystemLibrary.Delay` 0.2)
      (`self.ChasePlayer`))))

(event `Attack`
  (`|PlayMontage` (`self.Mesh`)
    (:`OnCompleted`
      _)
    (:`OnInterrupted`
      _))
  (`self.OnAttackEnd`))

(event `self.Box.OnComponentBeginOverlap`
  (params (OverlappedComponent :type "PrimitiveComponent Object Reference") (OtherActor :type "Actor Object Reference") (OtherComp :type "PrimitiveComponent Object Reference") (OtherBodyIndex :type Integer) (bFromSweep :type Boolean) (SweepResult :type "HitResult Structure (by ref)"))
  (cast `/Game/ThirdPerson/Blueprints/BP_ThirdPersonCharacter` OtherActor
    (:`then`
      (`self.K2_DestroyActor` (`GameplayStatics.GetPlayerController` 0))
      (bind _returnvalue (`|CreateWidget` "/Game/UI/Menues/MuerteMenu.MuerteMenu_C"))
      (`UserWidget.AddToViewport` _returnvalue 0))
    (:`CastFailed`
      (`KismetSystemLibrary.PrintString` "fafsafsaf"))))

(fn `GetPatrolRoute`
  (returns (PatrolRoute :type "/Game/Characters/MadeInIndia/Bp_PatrolRoute Object Reference"))
  (return (`self.PatrolRoute`)))

(fn `SetMovementSpeed`
  (params (Speed :type "/Game/Characters/MadeInIndia/AI/Enums/E_MovementSpeed Enum" :default "NewEnumerator0"))
  (returns (SpeedValue :type "Float (double-precision)"))
  (bind _output_get (set `CharacterMovementComponent.MaxWalkSpeed` (select `/Game/Characters/MadeInIndia/AI/Enums/E_MovementSpeed` Speed :`NewEnumerator1` 200.0 :`NewEnumerator2` 220.0 :`NewEnumerator3` 250.0 :!type "Float (single-precision)") (`self.CharacterMovement`)))
  (return _output_get))

(fn `UserConstructionScript`)