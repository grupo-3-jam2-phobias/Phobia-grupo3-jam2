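; Enemy character that wanders the navmesh and moves toward any pawn it sees.
; A self-calling event picks a random reachable point within a small radius and uses a retriggerable delay before each AI MoveTo.
; PawnSensing plays a walk animation once, sets walk speed and issues a move to the seen pawn.
; That move's Then output, not its success result, leads after a delay back into wandering.
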(event `self.ReceiveBeginPlay`
  (`self.Move Random Location`))

(event `Move Random Location`
  (bind _randomlocation (`NavigationSystemV1.K2_GetRandomLocationInNavigableRadius` (`self.K2_GetActorLocation`) 50.0 null null))
  (`KismetSystemLibrary.RetriggerableDelay` 2.0)
  (`|AIMoveTo` self _randomlocation null
    (:`then`
      (`self.Move Random Location`))))

(event `self.PawnSensing.OnSeePawn`
  (params (Pawn :type "Pawn Object Reference"))
  (`|ExecutionSequence`
    (:`then_0`
      (`SkeletalMeshComponent.PlayAnimation` (`self.Mesh`) "/Engine/Tutorial/SubEditors/TutorialAssets/Character/Tutorial_Walk_Fwd.Tutorial_Walk_Fwd" false)
      (set `CharacterMovementComponent.MaxWalkSpeed` 600.0 (`self.CharacterMovement`)))
    (:`then_1`
      (`|AIMoveTo` self (0.0 0.0 0.0) Pawn
        (:`then`
          (`KismetSystemLibrary.RetriggerableDelay` 2.0)
          (`SkeletalMeshComponent.PlayAnimation` (`self.Mesh`) "/Engine/Tutorial/SubEditors/TutorialAssets/Character/Tutorial_Walk_Fwd.Tutorial_Walk_Fwd" false)
          (set `CharacterMovementComponent.MaxWalkSpeed` 600.0 (`self.CharacterMovement`))
          (`self.Move Random Location`))))))

(fn `UserConstructionScript`)